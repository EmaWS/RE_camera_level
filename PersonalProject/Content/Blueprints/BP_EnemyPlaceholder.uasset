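; Placeholder enemy actor that takes a random element and is destroyed when it takes any damage.
; The construction script picks one of three entries from ElementTags at random and sets it as the actor's only tag.
; It then creates a dynamic instance of M_TestElement on the mesh and tints its Color to match the Fire, Water or Plant tag.
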(event `self.ReceiveAnyDamage`
  (params (Damage :type "Float (single-precision)") (DamageType :type "DamageType Object Reference") (InstigatedBy :type "Controller Object Reference") (DamageCauser :type "Actor Object Reference"))
  (`self.K2_DestroyActor`))

(fn `UserConstructionScript`
  (bind _mesh (`self.Mesh`))
  (bind _output_get (set `self.Tags` (`|MakeArray` (`|GetArrayItem` (`self.ElementTags`) (`KismetMathLibrary.RandomIntegerInRange` 0 2)))))
  (switch `name` (`|GetArrayItem` _output_get)
    (:`Fire`
      (bind _returnvalue (`PrimitiveComponent.CreateDynamicMaterialInstance` _mesh 0 "/Game/My_Materials/M_TestElement.M_TestElement" "None"))
      (`MaterialInstanceDynamic.SetVectorParameterValue` _returnvalue "Color" (make `LinearColor` 1.0 0.2 0.0 1.0)))
    (:`Water`
      (bind _returnvalue_2 (`PrimitiveComponent.CreateDynamicMaterialInstance` _mesh 0 "/Game/My_Materials/M_TestElement.M_TestElement" "None"))
      (`MaterialInstanceDynamic.SetVectorParameterValue` _returnvalue_2 "Color" (make `LinearColor` 0.2 0.2 1.0 1.0)))
    (:`Plant`
      (bind _returnvalue_3 (`PrimitiveComponent.CreateDynamicMaterialInstance` _mesh 0 "/Game/My_Materials/M_TestElement.M_TestElement" "None"))
      (`MaterialInstanceDynamic.SetVectorParameterValue` _returnvalue_3 "Color" (make `LinearColor` 0.0 0.6 0.0 1.0)))))
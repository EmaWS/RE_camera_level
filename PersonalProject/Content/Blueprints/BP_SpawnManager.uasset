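; BP_SpawnManager spawns BP_EnemyPlaceholder AI pawns and raises the allowed enemy count over time.
; A looping timer counts live enemies and, while below MaxEnemies, spawns one at a random point among five SpawnPointsRef entries.
; A 10-second timer increments MaxEnemies and updates its Looping flag against a limit of 20.
; That flag is read only when the timer is set, so changing it does not stop the timer.
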(event `self.ReceiveBeginPlay`
  (`KismetSystemLibrary.K2_SetTimerDelegate` (delegate `TryToSpawnEnemy`) (`self.Spawn Timer`) true)
  ;[1 1 1] Increase max enemies in scene every 10s
  (`KismetSystemLibrary.K2_SetTimerDelegate` (delegate `AddMaxEnemiesInScene`) 10.0 (`self.Looping`)))

(event `AddMaxEnemiesInScene`
  (bind _max_enemies (`self.Max Enemies`))
  ;[1 1 1] Increase max enemies in scene every 10s
  (`/Engine/EditorBlueprintResources/StandardMacros.IncrementInt` _max_enemies
    (:`  `
      (if (>= _max_enemies 20)
        (set `self.Looping` false)
        (else
          (set `self.Looping` true))))))

(event `TryToSpawnEnemy`
  ;[1 1 1] Check if you can spawn an enemy
  (bind _outactors (`GameplayStatics.GetAllActorsOfClass` "/Game/Blueprints/BP_EnemyPlaceholder.BP_EnemyPlaceholder_C"))
  (if (< (`KismetArrayLibrary.Array_Length` _outactors) (`self.Max Enemies`))
    (`self.Spawn Enemy`)))

(fn `UserConstructionScript`)
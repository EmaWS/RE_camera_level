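; A test damage box actor that damages the first-person character once each time it enters the box.
; Beginning an overlap applies Damage through a DoOnce gate, which resets when the character ends the overlap.
; On BeginPlay it passes ThisGameTag to the UI_NameTag inside its widget component, whose shadow casting is turned off there and in the construction script.
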(event `self.CollisionComponent.OnComponentBeginOverlap`
  (params (OverlappedComponent :type "PrimitiveComponent Object Reference") (OtherActor :type "Actor Object Reference") (OtherComp :type "PrimitiveComponent Object Reference") (OtherBodyIndex :type Integer) (bFromSweep :type Boolean) (SweepResult :type "HitResult Structure (by ref)"))
  (bind _asbp_first_person_character (cast `/Game/FirstPerson/Blueprints/BP_FirstPersonCharacter` OtherActor))
  (`/Engine/EditorBlueprintResources/StandardMacros.DoOnce` false :!label _label
    (:`Completed`
      (`GameplayStatics.ApplyDamage` _asbp_first_person_character (`self.Damage`)))))

(event `self.CollisionComponent.OnComponentEndOverlap`
  (params (OverlappedComponent :type "PrimitiveComponent Object Reference") (OtherActor :type "Actor Object Reference") (OtherComp :type "PrimitiveComponent Object Reference") (OtherBodyIndex :type Integer))
  (cast `/Game/FirstPerson/Blueprints/BP_FirstPersonCharacter` OtherActor)
  (goto _label :!via `Reset`))

(event `self.ReceiveBeginPlay`
  (`self.SetNameTag` (`self.ThisGameTag`)
    (:`Out`
      (`PrimitiveComponent.SetCastShadow` (`self.NameTagWidget`) false))))

(fn `UserConstructionScript`
  (`PrimitiveComponent.SetCastShadow` (`self.NameTagWidget`) false))
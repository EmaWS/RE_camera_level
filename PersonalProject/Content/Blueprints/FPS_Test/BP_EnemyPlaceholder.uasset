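; Placeholder FPS test enemy that endlessly chases the player through a looping AI MoveTo and shows a health bar widget.
; Construction script picks a random element tag and tints a dynamic material to match Fire, Water or Plant.
; Damage, NoDamage and Heal events update health and push it to UI_EnemyLife, with damage destroying the actor only at nearly zero health.
; Logic to turn the health bar toward the camera is unconnected.
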(event `self.ReceiveBeginPlay`
  ;[1 1 1] Set variabili "tra blueprint"
  ;;[0 0.1011 1] Appena il nemico spawna associo le variabili in "UI_EnemyLife" a quelle presenti qui (self).
  (bind _asui_enemy_life (cast `/Game/UI/UI_EnemyLife` (`WidgetComponent.GetUserWidgetObject` (`self.HealthBarWidget`))))
  (bind _output_get (set `self.WBP UI Enemy Life` _asui_enemy_life))
  (set `/Game/UI/UI_EnemyLife.UI Max Health` (`self.Max Health `) _output_get)
  (set `/Game/UI/UI_EnemyLife.UI Current Health` (`self.Current Health`) _output_get)
  ;[1 1 1] AI Follow
  (`|AIMoveTo` self (0.0 0.0 0.0) (`GameplayStatics.GetPlayerCharacter` 0) 100.0 :!label _label
    (:`OnSuccess`
      (`KismetSystemLibrary.Delay` 1.0)
      (goto _label))
    (:`OnFail`
      (`KismetSystemLibrary.Delay` 0.2)
      (goto _label))))

(event `self.ReceiveAnyDamage`
  (params (Damage :type "Float (single-precision)") (DamageType :type "DamageType Object Reference") (InstigatedBy :type "Controller Object Reference") (DamageCauser :type "Actor Object Reference"))
  (bind _returnvalue (- (`self.Current Health`) Damage))
  ;[1 1 1] Any Damage Event
  (`/Game/UI/UI_EnemyLife.Update Health` (`self.WBP UI Enemy Life`) _returnvalue)
  (bind _output_get (set `self.Current Health` _returnvalue))
  (`KismetSystemLibrary.PrintString` (`KismetStringLibrary.Conv_DoubleToString` _output_get))
  (if (`KismetMathLibrary.NearlyEqual_FloatFloat` _output_get)
    (`self.K2_DestroyActor`)))

(event `No Damage`
  (bind _returnvalue (- (`self.Current Health`) 0.0))
  ;[1 1 1] No Damage Event
  (`/Game/UI/UI_EnemyLife.Update Health` (`self.WBP UI Enemy Life`) _returnvalue)
  (bind _output_get (set `self.Current Health` _returnvalue))
  (`KismetSystemLibrary.PrintString` (`KismetStringLibrary.Conv_DoubleToString` _output_get)))

(event `Heal`
  (bind _returnvalue (+ (`self.Current Health`) 20.0))
  ;[1 1 1] Heal Event
  (if (not (>= (`self.Current Health`) 200.0))
    ;;[0 0.01166 1] Fondamentale, visto che l'unica variabile che fa cambiare la barra della vita effettiva è la vita attuale. Infatti in "UI_ecc" è presente questo evento (update health) che ad ogni cambiamento qui lo va a comunicare alla BP "UI_ecc" modificando il riempimento della barra.
    (`/Game/UI/UI_EnemyLife.Update Health` (`self.WBP UI Enemy Life`) _returnvalue)
    (bind _output_get (set `self.Current Health` _returnvalue))
    (`KismetSystemLibrary.PrintString` (`KismetStringLibrary.Conv_DoubleToString` _output_get))))

(fn `UserConstructionScript`
  (bind _meshcomponent (`self.MeshComponent`))
  (bind _output_get (set `self.Tags` (`|MakeArray` (`|GetArrayItem` (`self.ElementTags`) (`KismetMathLibrary.RandomIntegerInRange` 0 2)))))
  (switch `name` (`|GetArrayItem` _output_get)
    (:`Fire`
      (bind _returnvalue (`PrimitiveComponent.CreateDynamicMaterialInstance` _meshcomponent 0 "/Game/My_Materials/M_TestElement.M_TestElement" "None"))
      (`MaterialInstanceDynamic.SetVectorParameterValue` _returnvalue "Color" (make `LinearColor` 1.0 0.2 0.0 1.0)))
    (:`Water`
      (bind _returnvalue_2 (`PrimitiveComponent.CreateDynamicMaterialInstance` _meshcomponent 0 "/Game/My_Materials/M_TestElement.M_TestElement" "None"))
      (`MaterialInstanceDynamic.SetVectorParameterValue` _returnvalue_2 "Color" (make `LinearColor` 0.2 0.2 1.0 1.0)))
    (:`Plant`
      (bind _returnvalue_3 (`PrimitiveComponent.CreateDynamicMaterialInstance` _meshcomponent 0 "/Game/My_Materials/M_TestElement.M_TestElement" "None"))
      (`MaterialInstanceDynamic.SetVectorParameterValue` _returnvalue_3 "Color" (make `LinearColor` 0.0 0.6 0.0 1.0)))))
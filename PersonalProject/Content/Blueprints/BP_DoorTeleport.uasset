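; BP_DoorTeleport is a door that moves the tank-controls player character to a linked TeleportPoint when the player interacts with it.
; Its trigger overlap enables input on entry and disables it on exit, so IA_Interaction is received only nearby.
; On interaction, a Sequence fades the camera out while a parallel delay teleports the player to the point's Billboard transform once the screen darkens, then fades back in.
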(event `self.Trigger.OnComponentBeginOverlap`
  (params (OverlappedComponent :type "PrimitiveComponent Object Reference") (OtherActor :type "Actor Object Reference") (OtherComp :type "PrimitiveComponent Object Reference") (OtherBodyIndex :type Integer) (bFromSweep :type Boolean) (SweepResult :type "HitResult Structure (by ref)"))
  (`self.EnableInput` (`GameplayStatics.GetPlayerController` 0))
  (`KismetSystemLibrary.PrintString` "Entrato nel trigger"))

(event `self.Trigger.OnComponentEndOverlap`
  (params (OverlappedComponent :type "PrimitiveComponent Object Reference") (OtherActor :type "Actor Object Reference") (OtherComp :type "PrimitiveComponent Object Reference") (OtherBodyIndex :type Integer))
  (`self.DisableInput` (`GameplayStatics.GetPlayerController` 0))
  (`KismetSystemLibrary.PrintString` "Uscito dal trigger"))

(event `EnhancedInput|/Game/ThirdPerson/Input/Actions/IA_Interaction`
  (params (ActionValue :type Boolean) (ElapsedSeconds :type "Float (double-precision)") (TriggeredSeconds :type "Float (double-precision)") (InputAction :type "InputAction Object Reference" :default "/Game/ThirdPerson/Input/Actions/IA_Interaction.IA_Interaction"))
  (bind _returnvalue (`GameplayStatics.GetPlayerCameraManager` 0))
  (bind _billboard (`/Game/Blueprints/BP_TeleportPoint.Billboard` (`self.TeleportPoint`)))
  (:`Triggered`
    (bind _asbp_tpc_tank_controls (cast `/Game/ThirdPerson/Blueprints/BP_TPC_TankControls` (`GameplayStatics.GetPlayerCharacter` 0)))
    (set `self.Player` _asbp_tpc_tank_controls)
    (`|ExecutionSequence`
      (:`then_0`
        (`KismetSystemLibrary.Delay` 0.5)
        (`self.K2_TeleportTo` (`self.Player`) (`SceneComponent.K2_GetComponentLocation` _billboard) (`SceneComponent.K2_GetComponentRotation` _billboard)))
      (:`then_1`
        (`PlayerCameraManager.StartCameraFade` :`self` _returnvalue :`ToAlpha` 1.0 :`Duration` 0.5 :`bHoldWhenFinished` true)
        (`KismetSystemLibrary.Delay` 1.0)
        (`PlayerCameraManager.StartCameraFade` :`self` _returnvalue :`FromAlpha` 1.0 :`ToAlpha` 0.0 :`Duration` 0.2 :`bHoldWhenFinished` true)))))

(fn `UserConstructionScript`)
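; BP_DoorTeleport is an interactable door that teleports the tank-controls player to its TeleportPoint and can be locked from one side.
; Trigger overlap toggles the door's input, so IA_Interaction only responds nearby.
; An open door unlocks its linked OtherSideDoorTeleport, then runs sound, delayed teleport and camera fade in parallel while player input is disabled.
; A locked door plays a sound and shows timed bottom text via the SetBottomText helper.
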(event `self.Trigger.OnComponentBeginOverlap`
  (params (OverlappedComponent :type "PrimitiveComponent Object Reference") (OtherActor :type "Actor Object Reference") (OtherComp :type "PrimitiveComponent Object Reference") (OtherBodyIndex :type Integer) (bFromSweep :type Boolean) (SweepResult :type "HitResult Structure (by ref)"))
  ;[1 1 1 0.2] Input Handler
  (`self.EnableInput` (`GameplayStatics.GetPlayerController` 0))
  (`KismetSystemLibrary.PrintString` "Entrato nel trigger"))

(event `self.Trigger.OnComponentEndOverlap`
  (params (OverlappedComponent :type "PrimitiveComponent Object Reference") (OtherActor :type "Actor Object Reference") (OtherComp :type "PrimitiveComponent Object Reference") (OtherBodyIndex :type Integer))
  ;[1 1 1 0.2] Input Handler
  (`self.DisableInput` (`GameplayStatics.GetPlayerController` 0))
  (`KismetSystemLibrary.PrintString` "Uscito dal trigger"))

(event `EnhancedInput|/Game/ThirdPerson/Input/Actions/IA_Interaction`
  (params (ActionValue :type Boolean) (ElapsedSeconds :type "Float (double-precision)") (TriggeredSeconds :type "Float (double-precision)") (InputAction :type "InputAction Object Reference" :default "/Game/ThirdPerson/Input/Actions/IA_Interaction.IA_Interaction"))
  (bind _returnvalue (`GameplayStatics.GetPlayerCameraManager` 0))
  (bind _othersidedoorteleport (`self.OtherSideDoorTeleport`))
  (bind _player (`self.Player`))
  (bind _billboard (`/Game/Blueprints/RE_project/BP_TeleportPoint.Billboard` (`self.TeleportPoint`)))
  (:`Triggered`
    (bind _asbp_tpc_tank_controls (cast `/Game/ThirdPerson/Blueprints/BP_TPC_TankControls` (`GameplayStatics.GetPlayerCharacter` 0)))
    (bind _output_get (set `self.Player` _asbp_tpc_tank_controls))
    (`self.DisableInput` _output_get (`GameplayStatics.GetPlayerController` 0))
    (if (`self.CanGoThrough?`)
      (`/Engine/EditorBlueprintResources/StandardMacros.IsValid` _othersidedoorteleport
        (:`Is Valid`
          ;[1 1 1 0.2] Unlock Oder Side Door
          (if (`self.FirstTimeUnlock?`)
            (`GameplayStatics.PlaySound2D` "/Game/Sound/Door_Unlocked.Door_Unlocked" 1.0 1.0 0.0 null null)
            (`self.Set Bottom Text` (`/Game/ThirdPerson/Blueprints/BP_TPC_TankControls.UI Ref` (`self.Player`)) "Door unlocked!")
            (set `self.FirstTimeUnlock?` false))
          (set `/Game/Blueprints/RE_project/BP_DoorTeleport.CanGoThrough?` true _othersidedoorteleport))
        (:`Is Not Valid`
          _))
      (`|ExecutionSequence`
        (:`then_0`
          (`GameplayStatics.PlaySound2D` (`self.Door Sound`) 1.0 1.0 0.0 null null)
          ;[1 1 1 0.2] Teleport Logic
          (`KismetSystemLibrary.Delay` 0.8)
          (`self.K2_TeleportTo` (`self.Player`) (`SceneComponent.K2_GetComponentLocation` _billboard) (`SceneComponent.K2_GetComponentRotation` _billboard)))
        (:`then_1`
          ;[1 1 1 0.288] Fade In-Out Effect
          (`PlayerCameraManager.StartCameraFade` :`self` _returnvalue :`ToAlpha` 1.0 :`Duration` 0.8 :`bHoldWhenFinished` true)
          (`KismetSystemLibrary.Delay` 1.0)
          (`PlayerCameraManager.StartCameraFade` :`self` _returnvalue :`FromAlpha` 1.0 :`Duration` 0.8 :`bHoldWhenFinished` true)))
      (`self.EnableInput` (`self.Player`) (`GameplayStatics.GetPlayerController` 0))
      (else
        ;[1 1 1 0.2] Locked Door
        (`/Engine/EditorBlueprintResources/StandardMacros.DoOnce` false :!label _label
          (:`Completed`
            (`GameplayStatics.PlaySound2D` "/Game/Sound/DoorLocked.DoorLocked" 1.0 1.0 0.0 null null)
            (`self.Set Bottom Text` (`/Game/ThirdPerson/Blueprints/BP_TPC_TankControls.UI Ref` _player) "The door is locked from the other side...")
            (`self.EnableInput` _player (`GameplayStatics.GetPlayerController` 0))
            (goto _label :!via `Reset`)))))))

(fn `UserConstructionScript`)
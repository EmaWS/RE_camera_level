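; Collectable pickup actor that the player collects by pressing Interact while inside its trigger.
; Trigger overlap enables or disables input on the actor, and the construction script applies a configurable mesh.
; On interaction, it increments the collectable count on the tank-controls character's UI, plays a sound and hides the mesh.
; It shows a formatted pickup message in the bottom text, clears it after a short delay and destroys itself.
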(event `self.Trigger.OnComponentBeginOverlap`
  (params (OverlappedComponent :type "PrimitiveComponent Object Reference") (OtherActor :type "Actor Object Reference") (OtherComp :type "PrimitiveComponent Object Reference") (OtherBodyIndex :type Integer) (bFromSweep :type Boolean) (SweepResult :type "HitResult Structure (by ref)"))
  ;[1 1 1 0.2] Input Handler
  (`self.EnableInput` (`GameplayStatics.GetPlayerController` 0))
  (`KismetSystemLibrary.PrintString` "Trigger Collectable In"))

(event `self.Trigger.OnComponentEndOverlap`
  (params (OverlappedComponent :type "PrimitiveComponent Object Reference") (OtherActor :type "Actor Object Reference") (OtherComp :type "PrimitiveComponent Object Reference") (OtherBodyIndex :type Integer))
  ;[1 1 1 0.2] Input Handler
  (`self.DisableInput` (`GameplayStatics.GetPlayerController` 0))
  (`KismetSystemLibrary.PrintString` "Trigger Collectable Out"))

(event `EnhancedInput|/Game/ThirdPerson/Input/Actions/IA_Interaction`
  (params (ActionValue :type Boolean) (ElapsedSeconds :type "Float (double-precision)") (TriggeredSeconds :type "Float (double-precision)") (InputAction :type "InputAction Object Reference" :default "/Game/ThirdPerson/Input/Actions/IA_Interaction.IA_Interaction"))
  (:`Triggered`
    (bind _asbp_tpc_tank_controls (cast `/Game/ThirdPerson/Blueprints/BP_TPC_TankControls` (`GameplayStatics.GetPlayerCharacter` 0)))
    (bind _ui_ref (`/Game/ThirdPerson/Blueprints/BP_TPC_TankControls.UI Ref` _asbp_tpc_tank_controls))
    (`/Engine/EditorBlueprintResources/StandardMacros.IsValid` _ui_ref
      (:`Is Valid`
        (`/Engine/EditorBlueprintResources/StandardMacros.IncrementInt` (`/Game/UI_RE/UI_BottomText.NumberOfCollectables` _ui_ref)
          (:`  `
            (`GameplayStatics.PlaySound2D` "/Game/Sound/PickUp.PickUp" 1.0 1.0 0.0 null null)
            (`SceneComponent.SetVisibility` (`self.CollectableMesh`) false false)
            (set `/Game/UI_RE/UI_BottomText.BottomText` (`|FormatText` "{Main Text} {Object Name}" (`self.MainText`) (`self.StaticMeshName`)) _ui_ref)
            (`KismetSystemLibrary.Delay` 1.5)
            (set `/Game/UI_RE/UI_BottomText.BottomText` "" _ui_ref)
            (`self.K2_DestroyActor`)))))))

(fn `UserConstructionScript`
  (`StaticMeshComponent.SetStaticMesh` (`self.CollectableMesh`) (`self.New Mesh`)))
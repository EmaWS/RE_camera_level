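; BP_Lock is a lock interactable that reveals a static mesh when the player has the matching key.
; A trigger overlap enables player 0's input on the actor, and leaving the trigger disables it.
; On IA_Interaction, it casts the player character to BP_TPC_TankControls and compares KeyNameA to its own LockNameA.
; A match makes the mesh visible, while a mismatch prints a hint that something is needed.
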(event `self.Trigger.OnComponentBeginOverlap`
  (params (OverlappedComponent :type "PrimitiveComponent Object Reference") (OtherActor :type "Actor Object Reference") (OtherComp :type "PrimitiveComponent Object Reference") (OtherBodyIndex :type Integer) (bFromSweep :type Boolean) (SweepResult :type "HitResult Structure (by ref)"))
  (`self.EnableInput` (`GameplayStatics.GetPlayerController` 0)))

(event `self.Trigger.OnComponentEndOverlap`
  (params (OverlappedComponent :type "PrimitiveComponent Object Reference") (OtherActor :type "Actor Object Reference") (OtherComp :type "PrimitiveComponent Object Reference") (OtherBodyIndex :type Integer))
  (`self.DisableInput` (`GameplayStatics.GetPlayerController` 0)))

(event `EnhancedInput|/Game/ThirdPerson/Input/Actions/IA_Interaction`
  (params (ActionValue :type Boolean) (ElapsedSeconds :type "Float (double-precision)") (TriggeredSeconds :type "Float (double-precision)") (InputAction :type "InputAction Object Reference" :default "/Game/ThirdPerson/Input/Actions/IA_Interaction.IA_Interaction"))
  (:`Triggered`
    (bind _asbp_tpc_tank_controls (cast `/Game/ThirdPerson/Blueprints/BP_TPC_TankControls` (`GameplayStatics.GetPlayerCharacter` 0)))
    (if (== (`/Game/ThirdPerson/Blueprints/BP_TPC_TankControls.KeyName_A` _asbp_tpc_tank_controls) (`self.LockName_A`))
      (`SceneComponent.SetVisibility` (`self.StaticMesh`) true false)
      (else
        (`KismetSystemLibrary.PrintString` "I need something..." true true (struct :`G` 1.0 :`B` 0.875829 :`A` 1.0))))))

(fn `UserConstructionScript`)
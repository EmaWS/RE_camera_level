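; BP_Key is a key pickup that the player collects with the interaction input while inside its trigger.
; Trigger overlap events enable and disable input on the actor for player controller 0, without checking which actor overlaps.
; Interacting writes the key's name to KeyNameA on the BP_TPC_TankControls character and shows a found message through its UI reference.
; After a short delay it clears the message and destroys itself.
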(event `self.Trigger.OnComponentBeginOverlap`
  (params (OverlappedComponent :type "PrimitiveComponent Object Reference") (OtherActor :type "Actor Object Reference") (OtherComp :type "PrimitiveComponent Object Reference") (OtherBodyIndex :type Integer) (bFromSweep :type Boolean) (SweepResult :type "HitResult Structure (by ref)"))
  ;[1 1 1 0.2] Input Handler
  (`self.EnableInput` (`GameplayStatics.GetPlayerController` 0)))

(event `self.Trigger.OnComponentEndOverlap`
  (params (OverlappedComponent :type "PrimitiveComponent Object Reference") (OtherActor :type "Actor Object Reference") (OtherComp :type "PrimitiveComponent Object Reference") (OtherBodyIndex :type Integer))
  ;[1 1 1 0.2] Input Handler
  (`self.DisableInput` (`GameplayStatics.GetPlayerController` 0)))

(event `EnhancedInput|/Game/ThirdPerson/Input/Actions/IA_Interaction`
  (params (ActionValue :type Boolean) (ElapsedSeconds :type "Float (double-precision)") (TriggeredSeconds :type "Float (double-precision)") (InputAction :type "InputAction Object Reference" :default "/Game/ThirdPerson/Input/Actions/IA_Interaction.IA_Interaction"))
  (bind _keyname (`self.KeyName`))
  (:`Triggered`
    (bind _asbp_tpc_tank_controls (cast `/Game/ThirdPerson/Blueprints/BP_TPC_TankControls` (`GameplayStatics.GetPlayerCharacter` 0)))
    (set `/Game/ThirdPerson/Blueprints/BP_TPC_TankControls.KeyName_A` _keyname _asbp_tpc_tank_controls)
    (bind _ui_ref (`/Game/ThirdPerson/Blueprints/BP_TPC_TankControls.UI Ref` _asbp_tpc_tank_controls))
    (set `/Game/UI_RE/UI_BottomText.BottomText` (`|FormatText` "I found a {Key Name}" _keyname) _ui_ref)
    (`KismetSystemLibrary.Delay` 1.5)
    (set `/Game/UI_RE/UI_BottomText.BottomText` "" _ui_ref)
    (`self.K2_DestroyActor`)))

(fn `UserConstructionScript`)
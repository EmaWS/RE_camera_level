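; BP_Inspection is an interactable that lets the tank-controls player examine something or read a document.
; Its trigger overlap enables and disables input on the actor, so the interaction action only responds nearby.
; IsInspection selects between a sound with brief bottom-screen text, guarded by a DoOnce against spamming, and toggling a document widget showing NotesText.
; Player input is disabled while the document is open.
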(event `self.Trigger.OnComponentBeginOverlap`
  (params (OverlappedComponent :type "PrimitiveComponent Object Reference") (OtherActor :type "Actor Object Reference") (OtherComp :type "PrimitiveComponent Object Reference") (OtherBodyIndex :type Integer) (bFromSweep :type Boolean) (SweepResult :type "HitResult Structure (by ref)"))
  ;[1 1 1 0.2] Input Handler
  (`self.EnableInput` (`GameplayStatics.GetPlayerController` 0)))

(event `self.Trigger.OnComponentEndOverlap`
  (params (OverlappedComponent :type "PrimitiveComponent Object Reference") (OtherActor :type "Actor Object Reference") (OtherComp :type "PrimitiveComponent Object Reference") (OtherBodyIndex :type Integer))
  ;[1 1 1 0.2] Input Handler
  (`self.DisableInput` (`GameplayStatics.GetPlayerController` 0)))

(event `EnhancedInput|/Game/ThirdPerson/Input/Actions/IA_Interaction`
  (params (ActionValue :type Boolean) (ElapsedSeconds :type "Float (double-precision)") (TriggeredSeconds :type "Float (double-precision)") (InputAction :type "InputAction Object Reference" :default "/Game/ThirdPerson/Input/Actions/IA_Interaction.IA_Interaction"))
  (bind _returnvalue (`GameplayStatics.GetPlayerController` 0))
  (bind _player (`self.Player`))
  (:`Triggered`
    (bind _asbp_tpc_tank_controls (cast `/Game/ThirdPerson/Blueprints/BP_TPC_TankControls` (`GameplayStatics.GetPlayerCharacter` 0)))
    (bind _output_get (set `self.Player` _asbp_tpc_tank_controls))
    (if (`self.isInspection?`)
      ;[1 1 1 0.2] Inspection Logic
      (`/Engine/EditorBlueprintResources/StandardMacros.DoOnce` false :!label _label
        (:`Completed`
          (`GameplayStatics.PlaySound2D` "/Game/Sound/mmh__woman_.mmh__woman_" 1.0 1.0 0.0 null null)
          (bind _ui_ref (`/Game/ThirdPerson/Blueprints/BP_TPC_TankControls.UI Ref` _output_get))
          (set `/Game/UI_RE/UI_BottomText.BottomText` (`self.Main Text`) _ui_ref)
          (`KismetSystemLibrary.Delay` 1.5)
          (set `/Game/UI_RE/UI_BottomText.BottomText` "" _ui_ref)
          (goto _label :!via `Reset`)))
      (else
        ;[1 1 1 0.2] Document Inspection Logic
        (if (`self.isDocumentOnScreen?`)
          (bind _ui_document_ref (`/Game/ThirdPerson/Blueprints/BP_TPC_TankControls.UI Document Ref` _output_get))
          (`Widget.RemoveFromParent` _ui_document_ref)
          (set `self.isDocumentOnScreen?` false)
          (`self.EnableInput` _player _returnvalue)
          (else
            (`/Game/UI_RE/UI_Notes.SetDocumentText` _ui_document_ref (`self.NotesText`))
            (`UserWidget.AddToViewport` _ui_document_ref 0)
            (set `self.isDocumentOnScreen?` true)
            (`self.DisableInput` _player _returnvalue)))))))

(fn `UserConstructionScript`)